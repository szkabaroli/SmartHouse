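; Preview actor for the 3D preview feature that shows a static mesh scaled to fit and rotatable by mouse drag.
; SetMesh swaps the ViewMesh mesh, resets positions, then calls UpdateScale to uniformly fit its bounds within DesiredExtend and offset it toward its bounds center.
; Click start and end events toggle rotation, while mouse moves turn RenderScene in yaw and pitch by the cursor delta since the last update.
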(event Custom|UpdateScale
  (bind _viewmesh (Variables|Default|GetViewMesh))
  (bind _desiredextend (Variables|Default|GetDesiredExtend))
  (bind (_x _y _z) (Math|Vector|BreakVector _desiredextend))
  (bind (_origin _boxextent) (Collision|GetComponentBounds _viewmesh))
  (Variables|Default|SetCurrentExtendedMesh _boxextent)
  (Transformation|SetWorldScale3D _viewmesh (* (Transformation|GetWorldScale _viewmesh) (Math|Float|Min(Float) (/ _x (.X (Math|Vector|BreakVector (Variables|Default|GetCurrentExtendedMesh)))) (/ _y (.Y (Math|Vector|BreakVector (Variables|Default|GetCurrentExtendedMesh)))) (/ _z (.Z (Math|Vector|BreakVector (Variables|Default|GetCurrentExtendedMesh)))))))
  (Transformation|AddLocalOffset _viewmesh (- (Transformation|GetWorldLocation _viewmesh) _origin) false false))

(event Custom|OnMouseMove
  (params (MouseLocation :type Vector%202D%20Structure))
  (if (Variables|Default|Get?RotationEnabled)
    (Transformation|AddWorldRotation (Variables|Default|GetRenderScene) (Math|Rotator|MakeRotator 0.0 (.Y (Math|Vector2D|BreakVector2D (- MouseLocation (Variables|Default|GetOnStartRotateLocation)))) (/ (* (.X (Math|Vector2D|BreakVector2D (- MouseLocation (Variables|Default|GetOnStartRotateLocation)))) -1.0) 1.0)) false false)
    (Variables|Default|SetOnStartRotateLocation MouseLocation)))

(event Custom|OnClickStart
  (params (MouseLocation :type Vector%202D%20Structure))
  (Variables|Default|SetOnStartRotateLocation MouseLocation)
  (Variables|Default|Set?RotationEnabled true))

(event Custom|OnClickEnd
  (params (MouseLocation :type Vector%202D%20Structure))
  (Variables|Default|Set?RotationEnabled false))

(fn ConstructionScript)

(fn SetMesh
  (params (NewMesh :type Static%20Mesh%20Object%20Reference))
  (bind _viewmesh (Variables|Default|GetViewMesh))
  (Components|StaticMesh|SetStaticMesh _viewmesh NewMesh)
  (Transformation|SetRelativeLocation _viewmesh "0, 0, 0" false false)
  (Transformation|SetRelativeLocation (Variables|Default|GetRenderScene) "0, 0, 0" false false)
  (CallFunction|UpdateScale))