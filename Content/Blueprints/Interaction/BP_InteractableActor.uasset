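; BP_InteractableActor is an interactable actor with a configurable mesh and a widget that shows interaction text.
; The construction script applies the mesh, its offset and scale, and the widget offset.
; ShowText and HideText use two cross-resetting DoOnce gates to set the description or clear it once per change, printing debug strings.
; SetupUIText and ToggleHighlight are empty stubs.
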(event Custom|ShowText
  (bind _interactionui (Variables|UI|GetInteractionUI))
  (bind _returnvalue (UserInterface|GetUserWidgetObject _interactionui))
  (Utilities|FlowControl|Sequence
    (:then_0
      (Utilities|FlowControl|DoOnce false) ; enters at Reset
    )
    (:then_1
      (Utilities|FlowControl|DoOnce false
        (:Completed
          (UI|SetupUIText)
          (bind _asw_interaction_ui (Utilities|Casting|CastToW_InteractionUI _returnvalue))
          (Default|SetInteractionText _asw_interaction_ui (Variables|UI|GetUIDescription))
          (Development|PrintString "show"))))))

(event Custom|HideText
  (bind _interactionui (Variables|UI|GetInteractionUI))
  (bind _returnvalue (UserInterface|GetUserWidgetObject _interactionui))
  (Utilities|FlowControl|Sequence
    (:then_0
      (Utilities|FlowControl|DoOnce false) ; enters at Reset
    )
    (:then_1
      (Utilities|FlowControl|DoOnce false
        (:Completed
          (UI|SetupUIText)
          (bind _asw_interaction_ui (Utilities|Casting|CastToW_InteractionUI _returnvalue))
          (Default|SetInteractionText _asw_interaction_ui)
          (Development|PrintString "hide"))))))

(fn ConstructionScript
  (UI|SetupInteractionUI)
  (Interaction|SetupMesh))

(fn SetupInteractionUI
  (Transformation|SetRelativeLocation (Variables|UI|GetInteractionUI) (Variables|UI|GetUIOffset) false false))

(fn SetupUIText)

(fn ToggleHighlight)

(fn SetupMesh
  (Components|StaticMesh|SetStaticMesh (Variables|Default|GetIteractableMesh) (Variables|Mesh|GetActorMesh))
  (Transformation|SetRelativeLocation (Variables|Default|GetIteractableMesh) (Variables|Mesh|GetMeshOffset) false false)
  (Transformation|SetWorldScale3D (Variables|Default|GetIteractableMesh) (Variables|Mesh|GetMeshScale)))